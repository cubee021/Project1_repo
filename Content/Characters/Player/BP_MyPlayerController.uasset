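; Player controller that switches the player between the main dealer and sub dealer characters with the 1 and 2 keys.
; Each key first checks that the player is not already that class.
; It then saves the pawn's transform, destroys the pawn, spawns the chosen Blueprint at that transform and possesses it.
; Each switch creates a fresh actor, and no other pawn state is copied across.
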(event EventBeginPlay)

(event EventTick
  (params (DeltaSeconds :type Float%20%28single-precision%29)))

(event Input|KeyboardEvents|1
  (params (Key :type Key%20Structure :default "None"))
  (bind _returnvalue (Game|Player|GetPlayerPawn 0))
  ;[0.15 0.15 0.15 0.5] 메인딜러 -> 서브딜러
  (:Pressed
    (if (not (Class|GameplayStatics|ObjectIsA (Game|GetPlayerCharacter 0) "/Game/Characters/Player/MainDealer/BP_MainDealer.BP_MainDealer_C"))
      (bind _output_get (Variables|Default|SetOldPawnTransform (Transformation|GetActorTransform _returnvalue)))
      (Actor|DestroyActor _returnvalue)
      (bind _returnvalue_2 (Game|SpawnActorfromClass "/Game/Characters/Player/MainDealer/BP_MainDealer.BP_MainDealer_C" _output_get "Undefined" "MultiplyWithRoot" 0 0))
      (Pawn|Possess _returnvalue_2))))

(event Input|KeyboardEvents|2
  (params (Key :type Key%20Structure :default "None"))
  (bind _returnvalue (Game|Player|GetPlayerPawn 0))
  ;[0.15 0.15 0.15 0.5] 서브딜러 -> 메인딜러
  (:Pressed
    (if (not (Class|GameplayStatics|ObjectIsA (Game|GetPlayerCharacter 0) "/Game/Characters/Player/SubDealer/BP_SubDealer.BP_SubDealer_C"))
      (bind _output_get (Variables|Default|SetOldPawnTransform (Transformation|GetActorTransform _returnvalue)))
      (Actor|DestroyActor _returnvalue)
      (bind _returnvalue_2 (Game|SpawnActorfromClass "/Game/Characters/Player/SubDealer/BP_SubDealer.BP_SubDealer_C" _output_get "Undefined" "MultiplyWithRoot" 0 0))
      (Pawn|Possess _returnvalue_2))))

(fn ConstructionScript)