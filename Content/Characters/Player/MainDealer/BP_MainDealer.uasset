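; BP_MainDealer is a player character Blueprint that adds a melee-style area hit check to the inherited basic attack.
; Its BasicAttack override calls the parent, then runs the AttackCheck event.
; AttackCheck sphere-overlaps Pawns around the AttackSphere component using AttackRange, ignoring itself, and applies fixed damage to each one found.
; It also draws a temporary red debug sphere showing the hit area.
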(event Custom|AttackCheck
  (bind _attacksphere (Variables|Default|GetAttackSphere))
  (bind _attackrange (Variables|Default|GetAttackRange))
  (bind _returnvalue (Transformation|GetWorldLocation _attacksphere))
  ;[0.15 0.15 0.15 0.5] 공격 판정
  (bind _outactors (Collision|SphereOverlapActors _returnvalue _attackrange (Utilities|Array|MakeArray "ObjectTypeQuery3") 0 (Utilities|Array|MakeArray self)))
  (Rendering|Debug|DrawDebugSphere _returnvalue _attackrange 12 "(R=1.000000,G=0.011672,B=0.000000,A=1.000000)" 2.0)
  (for _array_element _outactors
    (Game|Damage|ApplyDamage _array_element 1e+01 (Pawn|GetController) self)))

(event EventBeginPlay
  (|CallParentFunction) ; This node is disabled and will not be called.\nDrag off pins to build functionality.
)

(event Collision|EventActorBeginOverlap
  (params (OtherActor :type Actor%20Object%20Reference))
  (|CallParentFunction OtherActor) ; This node is disabled and will not be called.\nDrag off pins to build functionality.
)

(event EventTick
  (params (DeltaSeconds :type Float%20%28single-precision%29))
  (|CallParentFunction DeltaSeconds) ; This node is disabled and will not be called.\nDrag off pins to build functionality.
)

(fn ConstructionScript
  (|CallParentFunction))

(fn BasicAttack
  (|CallParentFunction)
  (CallFunction|AttackCheck))