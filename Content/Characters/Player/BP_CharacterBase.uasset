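; Player character base that switches between a melee main dealer and an arrow-shooting sub dealer by toggling mesh visibility.
; Enhanced Input drives movement, look, jump, dash and attacks, with montage-section combos that briefly lock movement.
; Delay-recursive events drain and regain dash stamina.
; Each dealer keeps separate health mirrored into display values; lethal damage triggers ragdoll, and F calls BP_Sword to start the boss battle.
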(event OnComponentBeginOverlap(CapsuleComponent)
  (params (OverlappedComponent :type Primitive%20Component%20Object%20Reference) (OtherActor :type Actor%20Object%20Reference) (OtherComp :type Primitive%20Component%20Object%20Reference) (OtherBodyIndex :type Integer) (bFromSweep :type Boolean) (SweepResult :type Hit%20Result%20Structure%20%28by%20ref%29))
  ;[0.15 0.15 0.15 0.5] 맵 상호작용
)

(event Custom|CustomEvent
  ;[0.15 0.15 0.15 0.5] 일반 공격
  ;;[0.15 0.15 0.15 0.5] 메인딜러
  (CallFunction|OnAnimEndAttack))

(event Custom|OnAnimEnd_Attack
  ;[0.15 0.15 0.15 0.5] 일반 공격
  ;;[0.15 0.15 0.15 0.5] 콤보 종료
  (Variables|Default|SetIsAttacking false)
  (Variables|Default|SetAttackIndex 0)
  (Variables|Default|SetIsGoNextCombo false))

(event Custom|OnAnim_CheckNextCombo
  ;[0.15 0.15 0.15 0.5] 일반 공격
  ;;[0.15 0.15 0.15 0.5] 콤보 판정
  (if (Variables|Default|GetIsGoNextCombo)
    (Variables|Default|SetIsGoNextCombo false)
    (bind _output_get (Variables|Default|SetAttackIndex (+ (Variables|Default|GetAttackIndex) 1)))
    (switch int _output_get
      (:1
        (Animation|PlayAnimMontage "/Game/Characters/Player/Animations/AM_ComboAttack.AM_ComboAttack" 1.0 "Attack1"))
      (:2
        (Animation|PlayAnimMontage "/Game/Characters/Player/Animations/AM_ComboAttack.AM_ComboAttack" 1.0 "Attack2")))
    ;[0.15 0.15 0.15 0.5] 애니메이션중 잠시 멈춤
    (Pawn|Components|CharacterMovement|DisableMovement (Variables|Character|GetCharacterMovement))
    (Utilities|Time|SetTimerbyEvent (delegate Custom|CustomEvent_1) 0.5)))

(event Custom|CustomEvent_1
  ;[0.15 0.15 0.15 0.5] 애니메이션중 잠시 멈춤
  (Pawn|Components|CharacterMovement|SetMovementMode (Variables|Character|GetCharacterMovement) "MOVE_Walking" 0))

(event Custom|RegainStamina
  ;[0.15 0.15 0.15 0.5] 대쉬
  ;;[0.15 0.15 0.15 0.5] 스태미나 회복
  (bind _output_get (Variables|Default|SetStamina (Math|Float|Clamp(Float) (+ (Variables|Default|GetStamina) 2.0) 0.0 (Variables|Default|GetMaxStamina))))
  (if (not (== _output_get (Variables|Default|GetMaxStamina)))
    (if (not (Variables|Default|GetIsDashing))
      (Utilities|FlowControl|Delay 0.1)
      (CallFunction|RegainStamina))))

(event Custom|DrainStamina
  ;[0.15 0.15 0.15 0.5] 대쉬
  ;;[0.15 0.15 0.15 0.5] 스태미나 감소
  (if (> (Math|Vector|VectorLength (Transformation|GetVelocity)) 0.0)
    (bind _output_get (Variables|Default|SetStamina (Math|Float|Clamp(Float) (- (Variables|Default|GetStamina) 1.0) 0.0 (Variables|Default|GetMaxStamina))))
    (if (== _output_get 0.0)
      (CallFunction|StopDashing)
      (elif (Variables|Default|GetIsDashing)
        (Utilities|FlowControl|Delay 0.1)
        (CallFunction|DrainStamina)))))

(event Custom|CustomEvent_0
  ;[0.15 0.15 0.15 0.5] 애니메이션중 잠시 멈춤
  (Pawn|Components|CharacterMovement|SetMovementMode (Variables|Character|GetCharacterMovement) "MOVE_Walking" 0))

(event Input|EnhancedActionEvents|EnhancedInputActionIA_PlayerLook
  (params (ActionValue :type Vector%202D%20Structure) (ElapsedSeconds :type Float%20%28double-precision%29) (TriggeredSeconds :type Float%20%28double-precision%29) (InputAction :type Input%20Action%20Object%20Reference :default "/Game/Characters/Player/Input/IA_PlayerLook.IA_PlayerLook"))
  ;[0.15 0.15 0.15 0.5] 카메라 회전
  (if (> (Math|Float|Absolute(Float) (.x ActionValue)) (Math|Float|Absolute(Float) (.y ActionValue)))
    (Pawn|Input|AddControllerYawInput (.x ActionValue))
    (else
      (Pawn|Input|AddControllerPitchInput (/ (.y ActionValue) 3.0)))))

(event Input|EnhancedActionEvents|EnhancedInputActionIA_PlayerMove
  (params (ActionValue :type Vector%202D%20Structure) (ElapsedSeconds :type Float%20%28double-precision%29) (TriggeredSeconds :type Float%20%28double-precision%29) (InputAction :type Input%20Action%20Object%20Reference :default "/Game/Characters/Player/Input/IA_PlayerMove.IA_PlayerMove"))
  (bind _returnvalue (Pawn|GetControlRotation :!class /Script/Engine.Pawn))
  ;[0.15 0.15 0.15 0.5] 움직임
  (Pawn|Input|AddMovementInput (Math|Vector|GetRightVector (Math|Rotator|MakeRotator (.roll _returnvalue) 0.0 (.yaw _returnvalue))) (.x ActionValue) false)
  (Pawn|Input|AddMovementInput (Math|Vector|GetForwardVector (Math|Rotator|MakeRotator 0.0 0.0 (.yaw (Pawn|GetControlRotation :!class /Script/Engine.Pawn)))) (.y ActionValue) false))

(event Input|EnhancedActionEvents|EnhancedInputActionIA_PlayerJump
  (params (ActionValue :type Boolean) (ElapsedSeconds :type Float%20%28double-precision%29) (TriggeredSeconds :type Float%20%28double-precision%29) (InputAction :type Input%20Action%20Object%20Reference :default "/Game/Characters/Player/Input/IA_PlayerJump.IA_PlayerJump"))
  ;[0.15 0.15 0.15 0.5] 점프
  (:Triggered
    (Character|Jump))
  (:Completed
    (Character|StopJumping)))

(event Input|EnhancedActionEvents|EnhancedInputActionIA_Dash
  (params (ActionValue :type Boolean) (ElapsedSeconds :type Float%20%28double-precision%29) (TriggeredSeconds :type Float%20%28double-precision%29) (InputAction :type Input%20Action%20Object%20Reference :default "/Game/Characters/Player/Input/IA_Dash.IA_Dash"))
  ;[0.15 0.15 0.15 0.5] 대쉬
  (:Triggered
    (CallFunction|StartDashing))
  (:Completed
    (CallFunction|StopDashing)))

(event Input|EnhancedActionEvents|EnhancedInputActionIA_BasicAttack
  (params (ActionValue :type Boolean) (ElapsedSeconds :type Float%20%28double-precision%29) (TriggeredSeconds :type Float%20%28double-precision%29) (InputAction :type Input%20Action%20Object%20Reference :default "/Game/Characters/Player/Input/IA_BasicAttack.IA_BasicAttack"))
  ;[0.15 0.15 0.15 0.5] 일반 공격
  (if (Variables|Default|GetIsMainDealer)
    ;;[0.15 0.15 0.15 0.5] 메인딜러
    (if (Variables|Default|GetIsAttacking)
      (Utilities|Time|SetTimerbyEvent (delegate Custom|CustomEvent) 0.4)
      (Variables|Default|SetIsGoNextCombo true)
      (else
        (Variables|Default|SetIsAttacking true)
        (Animation|PlayAnimMontage "/Game/Characters/Player/Animations/AM_ComboAttack.AM_ComboAttack" 1.0 "None")
        ;[0.15 0.15 0.15 0.5] 애니메이션중 잠시 멈춤
        (Pawn|Components|CharacterMovement|DisableMovement (Variables|Character|GetCharacterMovement))
        (Utilities|Time|SetTimerbyEvent (delegate Custom|CustomEvent_0) 0.5)))
    (else
      ;;[0.15 0.15 0.15 0.5] 서브딜러
      (Game|SpawnActorfromClass "/Game/Characters/Player/BP_Arrow.BP_Arrow_C" (Transformation|GetWorldTransform (Variables|Default|GetShootPoint)) "Undefined" "MultiplyWithRoot" 0 0))))

(event EventBeginPlay
  (bind _mainmaxhealth (Variables|Default|GetMainMaxHealth))
  ;[0.15 0.15 0.15 0.5] Enhanced Input Casting
  (bind _asplayer_controller (Utilities|Casting|CastToPlayerController (Pawn|GetController)))
  (Utilities|IsValid (PlayerController|LocalPlayerSubsystems|GetEnhancedInputLocalPlayerSubsystem _asplayer_controller)
    (:Is%20Valid
      (Input|AddMappingContext (PlayerController|LocalPlayerSubsystems|GetEnhancedInputLocalPlayerSubsystem _asplayer_controller) "/Game/Characters/Player/Input/IMC_PlayerInput.IMC_PlayerInput" 0 "(bIgnoreAllPressedKeysUntilRelease=True,bForceImmediately=False,bNotifyUserSettings=False)")
      ;[0.15 0.15 0.15 0.5] 서브딜러 숨기기
      (Development|SetHiddeninGame (Variables|Default|GetSubDealer) true false)
      (Variables|Default|SetIsMainDealer true)
      ;[0.15 0.15 0.15 0.5] Add Main UI
      (bind _returnvalue (UserInterface|CreateWidget "/Game/Characters/Player/UI/WB_MainUI.WB_MainUI_C"))
      (UserInterface|Viewport|AddtoViewport _returnvalue 0)
      ;[0.15 0.15 0.15 0.5] 메인딜러 Hp 초기화
      (Variables|Default|SetMainCurrentHealth _mainmaxhealth)
      (Variables|Default|SetMaxHpToView _mainmaxhealth)
      (Variables|Default|SetCurrentHpToView _mainmaxhealth)
      ;[0.15 0.15 0.15 0.5] 서브딜러 Hp 초기화
      (Variables|Default|SetSubCurrentHealth (Variables|Default|GetSubMaxHealth)))))

(event Collision|EventActorBeginOverlap
  (params (OtherActor :type Actor%20Object%20Reference)))

(event EventTick
  (params (DeltaSeconds :type Float%20%28single-precision%29)))

(event Game|Damage|EventAnyDamage
  (params (Damage :type Float%20%28single-precision%29) (DamageType :type Damage%20Type%20Object%20Reference) (InstigatedBy :type Controller%20Object%20Reference) (DamageCauser :type Actor%20Object%20Reference))
  ;[0.15 0.15 0.15 0.5] Damage/Dead
  (CallFunction|ShowDamageAnim)
  (Variables|Default|SetDamageAmount Damage)
  (Variables|Default|SetCurrentHpToView (- (Variables|Default|GetCurrentHpToView) Damage))
  (CallFunction|UpdateSideBar)
  (if (<= (Variables|Default|GetCurrentHpToView) 0.0)
    (Pawn|Components|CharacterMovement|DisableMovement (Variables|Character|GetCharacterMovement))
    (Physics|SetSimulatePhysics (Variables|Character|GetMesh) true)))

(event Input|KeyboardEvents|1
  (params (Key :type Key%20Structure :default "None"))
  ;[0.15 0.15 0.15 0.5] 메인딜러 <-> 서브딜러
  (:Pressed
    (Development|SetHiddeninGame (Variables|Default|GetSubDealer) true false)
    (Development|SetHiddeninGame (Variables|Character|GetMesh) false false)
    (Variables|Default|SetIsMainDealer true)
    (CallFunction|SwitchHealth)))

(event Input|KeyboardEvents|2
  (params (Key :type Key%20Structure :default "None"))
  ;[0.15 0.15 0.15 0.5] 메인딜러 <-> 서브딜러
  (:Pressed
    (Development|SetHiddeninGame (Variables|Default|GetSubDealer) false false)
    (Development|SetHiddeninGame (Variables|Character|GetMesh) true false)
    (Variables|Default|SetIsMainDealer false)
    (CallFunction|SwitchHealth)))

(event Input|KeyboardEvents|F
  (params (Key :type Key%20Structure :default "None"))
  ;[0.15 0.15 0.15 0.5] 맵 상호작용
  (:Pressed
    (bind _asbp_sword (Utilities|Casting|CastToBP_Sword (stale OnComponentBeginOverlap(CapsuleComponent) OtherActor)))
    (bind _returnvalue (Actor|GetActorOfClass "BP_CharacterBase_C"))
    (Default|StartBossBattle _asbp_sword _returnvalue)
    (Actor|DestroyActor _asbp_sword)))

(fn ConstructionScript)

(fn StartDashing
  (Variables|/Script/Engine.CharacterMovementComponent|SetMaxWalkSpeed (Variables|Character|GetCharacterMovement) 1.2e+03)
  (Variables|Default|SetIsDashing true)
  (CallFunction|DrainStamina))

(fn StopDashing
  (Variables|/Script/Engine.CharacterMovementComponent|SetMaxWalkSpeed (Variables|Character|GetCharacterMovement) 5e+02)
  (Variables|Default|SetIsDashing false)
  (CallFunction|RegainStamina))

(fn ShowDamageAnim
  ;[0.15 0.15 0.15 0.5] 피격 당하면 damage 표시
  (bind _aswb_get_damage_widget (Utilities|Casting|CastToWB_GetDamageWidget (UserInterface|GetWidget (Variables|Default|GetDamageWidget))))
  (Widget|SetVisibility _aswb_get_damage_widget "Visible")
  (UserInterface|Animation|PlayAnimation _aswb_get_damage_widget (Variables|/Game/Characters/Player/UI/WB_GetDamageWidget.WB_GetDamageWidget_C|GetShowDamage _aswb_get_damage_widget) 0.0 1 "Forward" 1.0 false))

(fn SwitchHealth
  (if (Variables|Default|GetIsMainDealer)
    ;[0.15 0.15 0.15 0.5] 하단Hp바에 서브딜러 Hp 업데이트
    (Variables|Default|SetMaxHpToView (Variables|Default|GetMainMaxHealth))
    (Variables|Default|SetCurrentHpToView (Variables|Default|GetMainCurrentHealth))
    (else
      ;[0.15 0.15 0.15 0.5] 하단Hp바에 메인딜러 Hp 업데이트
      (Variables|Default|SetMaxHpToView (Variables|Default|GetSubMaxHealth))
      (Variables|Default|SetCurrentHpToView (Variables|Default|GetSubCurrentHealth)))))

(fn UpdateSideBar
  (if (Variables|Default|GetIsMainDealer)
    ;[0.15 0.15 0.15 0.5] 메인딜러 사이드바 업데이트
    (Variables|Default|SetMainCurrentHealth (- (Variables|Default|GetMainCurrentHealth) (Variables|Default|GetDamageAmount)))
    (else
      ;[0.15 0.15 0.15 0.5] 서브딜러 사이드바 업데이트
      (Variables|Default|SetSubCurrentHealth (- (Variables|Default|GetSubCurrentHealth) (Variables|Default|GetDamageAmount))))))