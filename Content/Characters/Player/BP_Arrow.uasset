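; BP_Arrow is a player arrow projectile that damages the boss on contact.
; Tick moves it along its forward vector at Speed, setting the location directly without sweep or a movement component.
; On overlap with BP_Boss it applies fixed damage and destroys itself after a short delay.
; Other overlaps are ignored, and the graph has no other destroy path.
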(event EventBeginPlay)

(event Collision|EventActorBeginOverlap
  (params (OtherActor :type Actor%20Object%20Reference))
  ;[0.15 0.15 0.15 0.5] 보스 피격
  (bind _asbp_boss (Utilities|Casting|CastToBP_Boss OtherActor))
  (Game|Damage|ApplyDamage _asbp_boss 5.0 0 0)
  (Utilities|FlowControl|Delay 0.2)
  (Actor|DestroyActor))

(event EventTick
  (params (DeltaSeconds :type Float%20%28single-precision%29))
  ;[0.15 0.15 0.15 0.5] 화살 앞으로
  (Transformation|SetActorLocation (+ (* DeltaSeconds (* (Variables|Default|GetSpeed) (Transformation|GetActorForwardVector))) (Transformation|GetActorLocation)) false false))

(fn ConstructionScript)