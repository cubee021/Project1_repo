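; Test player character with Enhanced Input movement, look and jump, plus a stamina-limited dash, an attack and health.
; BeginPlay adds the input mapping context and stamina widget.
; Dashing raises walk speed and toggles self-calling Delay loops that drain or regain stamina, stopping the dash at zero.
; Left mouse sphere-traces pawns from the camera to apply damage, with debug drawing; at zero health the character stops moving and ragdolls.
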(event Custom|RegainStamina
  ;[0.15 0.15 0.15 0.5] 대쉬
  ;;[0.15 0.15 0.15 0.5] 스태미나 회복
  (bind _output_get (Variables|Default|SetStamina (Math|Float|Clamp(Float) (+ (Variables|Default|GetStamina) 2.0) 0.0 (Variables|Default|GetMaxStamina))))
  (if (not (== _output_get (Variables|Default|GetMaxStamina)))
    (if (not (Variables|Default|GetIsDashing))
      (Utilities|FlowControl|Delay 0.1)
      (CallFunction|RegainStamina))))

(event Custom|DrainStamina
  ;[0.15 0.15 0.15 0.5] 대쉬
  ;;[0.15 0.15 0.15 0.5] 스태미나 감소
  (bind _output_get (Variables|Default|SetStamina (Math|Float|Clamp(Float) (- (Variables|Default|GetStamina) 0.3) 0.0 (Variables|Default|GetMaxStamina))))
  (if (== _output_get 0.0)
    (CallFunction|StopDashing)
    (elif (Variables|Default|GetIsDashing)
      (Utilities|FlowControl|Delay 0.1)
      (CallFunction|DrainStamina))))

(event Input|EnhancedActionEvents|EnhancedInputActionIA_PlayerLook
  (params (ActionValue :type Vector%202D%20Structure) (ElapsedSeconds :type Float%20%28double-precision%29) (TriggeredSeconds :type Float%20%28double-precision%29) (InputAction :type Input%20Action%20Object%20Reference :default "/Game/Characters/Player/Input/IA_PlayerLook.IA_PlayerLook"))
  ;[0.15 0.15 0.15 0.5] 카메라 회전
  (Pawn|Input|AddControllerYawInput (.x ActionValue))
  (Pawn|Input|AddControllerPitchInput (.y ActionValue)))

(event Input|EnhancedActionEvents|EnhancedInputActionIA_PlayerMove
  (params (ActionValue :type Vector%202D%20Structure) (ElapsedSeconds :type Float%20%28double-precision%29) (TriggeredSeconds :type Float%20%28double-precision%29) (InputAction :type Input%20Action%20Object%20Reference :default "/Game/Characters/Player/Input/IA_PlayerMove.IA_PlayerMove"))
  (bind _returnvalue (Pawn|GetControlRotation :!class /Script/Engine.Pawn))
  ;[0.15 0.15 0.15 0.5] 움직임
  (Pawn|Input|AddMovementInput (Math|Vector|GetRightVector (Math|Rotator|MakeRotator (.roll _returnvalue) 0.0 (.yaw _returnvalue))) (.x ActionValue) false)
  (Pawn|Input|AddMovementInput (Math|Vector|GetForwardVector (Math|Rotator|MakeRotator 0.0 0.0 (.yaw (Pawn|GetControlRotation :!class /Script/Engine.Pawn)))) (.y ActionValue) false))

(event Input|EnhancedActionEvents|EnhancedInputActionIA_PlayerJump
  (params (ActionValue :type Boolean) (ElapsedSeconds :type Float%20%28double-precision%29) (TriggeredSeconds :type Float%20%28double-precision%29) (InputAction :type Input%20Action%20Object%20Reference :default "/Game/Characters/Player/Input/IA_PlayerJump.IA_PlayerJump"))
  ;[0.15 0.15 0.15 0.5] 점프
  (:Triggered
    (Character|Jump))
  (:Completed
    (Character|StopJumping)))

(event Input|EnhancedActionEvents|EnhancedInputActionIA_Dash
  (params (ActionValue :type Boolean) (ElapsedSeconds :type Float%20%28double-precision%29) (TriggeredSeconds :type Float%20%28double-precision%29) (InputAction :type Input%20Action%20Object%20Reference :default "/Game/Characters/Player/Input/IA_Dash.IA_Dash"))
  ;[0.15 0.15 0.15 0.5] 대쉬
  (:Triggered
    (CallFunction|StartDashing))
  (:Completed
    (CallFunction|StopDashing)))

(event EventBeginPlay
  ;[0.15 0.15 0.15 0.5] Enhanced Input Casting
  (bind _asplayer_controller (Utilities|Casting|CastToPlayerController (Pawn|GetController)))
  (Utilities|IsValid (PlayerController|LocalPlayerSubsystems|GetEnhancedInputLocalPlayerSubsystem _asplayer_controller)
    (:Is%20Valid
      (Input|AddMappingContext (PlayerController|LocalPlayerSubsystems|GetEnhancedInputLocalPlayerSubsystem _asplayer_controller) "/Game/Characters/Player/Input/IMC_PlayerInput.IMC_PlayerInput" 0 "(bIgnoreAllPressedKeysUntilRelease=True,bForceImmediately=False,bNotifyUserSettings=False)")
      ;[0.15 0.15 0.15 0.5] Stamina Widget
      (bind _returnvalue (UserInterface|CreateWidget "/Game/Characters_testing/Player/UI/StaminaWidget_testing.StaminaWidget_testing_C"))
      (UserInterface|Viewport|AddtoViewport _returnvalue 0))))

(event Collision|EventActorBeginOverlap
  (params (OtherActor :type Actor%20Object%20Reference)))

(event EventTick
  (params (DeltaSeconds :type Float%20%28single-precision%29)))

(event Game|Damage|EventAnyDamage
  (params (Damage :type Float%20%28single-precision%29) (DamageType :type Damage%20Type%20Object%20Reference) (InstigatedBy :type Controller%20Object%20Reference) (DamageCauser :type Actor%20Object%20Reference))
  ;[0.15 0.15 0.15 0.5] Health
  (Variables|Default|Sethealth (- (Variables|Default|Gethealth) Damage))
  (if (<= (Variables|Default|Gethealth) 0.0)
    (Pawn|Components|CharacterMovement|DisableMovement (Variables|Character|GetCharacterMovement))
    (Physics|SetSimulatePhysics (Variables|Character|GetMesh) true)))

(event Input|MouseEvents|LeftMouseButton
  (params (Key :type Key%20Structure :default "None"))
  (bind _camera (Variables|Default|GetCamera))
  (bind _returnvalue (Transformation|GetWorldLocation _camera))
  ;[0.15 0.15 0.15 0.5] Attack
  (:Pressed
    (bind (_outhit _returnvalue_2) (Collision|SphereTraceForObjects _returnvalue (+ _returnvalue (* (Math|Vector|GetForwardVector (Transformation|GetWorldRotation _camera)) 3e+03)) 25.0 (Utilities|Array|MakeArray "ObjectTypeQuery3") false 0 "ForDuration" true "(R=1.000000,G=0.000000,B=0.000000,A=1.000000)" "(R=0.000000,G=1.000000,B=0.000000,A=1.000000)" 2.0))
    (if _returnvalue_2
      (Game|Damage|ApplyDamage (.HitActor (Collision|BreakHitResult _outhit)) 1e+01 0 0))))

(fn ConstructionScript)

(fn StartDashing
  (Variables|/Script/Engine.CharacterMovementComponent|SetMaxWalkSpeed (Variables|Character|GetCharacterMovement) 1e+03)
  (Variables|Default|SetIsDashing true)
  (CallFunction|DrainStamina))

(fn StopDashing
  (Variables|/Script/Engine.CharacterMovementComponent|SetMaxWalkSpeed (Variables|Character|GetCharacterMovement) 5e+02)
  (Variables|Default|SetIsDashing false)
  (CallFunction|RegainStamina))