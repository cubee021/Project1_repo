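; Boss attack component, owned by the boss AI controller, that implements an ice charge toward the player character.
; IceCharge first locks a normalized direction to BP_CharacterBase, then each subsequent call sweeps BP_Boss along it, scaled by delta time and charge speed.
; Once the charge time elapses, it changes the controller's AttackState, increments its attack count and resets for the next charge.
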(event EventBeginPlay)

(event EventTick
  (params (DeltaSeconds :type Float%20%28single-precision%29)))

(fn IceCharge
  (if (Variables|Default|GetIsAttackDirectionSet?)
    (bind _output_get (Variables|Default|SetIceChargeCurrentTime (+ (Variables|Default|GetIceChargeCurrentTime) (Utilities|Time|GetWorldDeltaSeconds))))
    (if (> _output_get (Variables|Default|GetIceChargeTime))
      (Development|PrintString "돌진끝@@@@@@@@@")
      (bind _asbp_boss_aicontroller (Utilities|Casting|CastToBP_BossAIController (Components|GetOwner)))
      (Variables|/Game/Boss/BP_BossAIController.BP_BossAIController_C|SetAttackState _asbp_boss_aicontroller "NewEnumerator5")
      (Development|PrintString "돌진끝@@@@@@")
      (Variables|/Game/Boss/BP_BossAIController.BP_BossAIController_C|SetCurrentAttackCount _asbp_boss_aicontroller (+ (Variables|/Game/Boss/BP_BossAIController.BP_BossAIController_C|GetCurrentAttackCount _asbp_boss_aicontroller) 1))
      (Variables|Default|SetIsAttackDirectionSet? false)
      (Variables|Default|SetIceChargeCurrentTime 0.0)
      (else
        (bind _returnvalue (Actor|GetActorOfClass "/Game/Boss/BP_Boss.BP_Boss_C"))
        (Transformation|SetActorTransform _returnvalue (Math|Transform|MakeTransform (+ (* (Utilities|Time|GetWorldDeltaSeconds) (* (Variables|Default|GetAttackDirection) (LocalVariables|GetBossIceChargeSpeed))) (Transformation|GetActorLocation _returnvalue)) (Math|Conversions|RotationFromXVector (Variables|Default|GetAttackDirection)) "1.000000,1.000000,1.000000") true)))
    (else
      (CallFunction|SetAttackDirection)
      (Variables|Default|SetIsAttackDirectionSet? true))))

(fn SetAttackDirection
  (bind _returnvalue (Actor|GetActorOfClass "/Game/Characters/Player/BP_CharacterBase.BP_CharacterBase_C"))
  (bind _returnvalue_2 (Actor|GetActorOfClass "/Game/Boss/BP_Boss.BP_Boss_C"))
  (Variables|Default|SetAttackDirection (Math|Vector|Normalize (- (Transformation|GetActorLocation _returnvalue) (Transformation|GetActorLocation _returnvalue_2))))
  (return))