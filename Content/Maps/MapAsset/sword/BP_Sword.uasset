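; BP_Sword is a sword actor that lets the player start a boss battle when nearby.
; It adds a WB_SwordWidget to the viewport on BeginPlay, and its capsule overlap shows it with a fade-in or fades it out and hides it after a short delay.
; StartBossBattle sets IsBattleReady on BP_MyGameModeBase only while the widget is visible, so widget visibility acts as the proximity gate.
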(event OnComponentBeginOverlap(Capsule)
  (params (OverlappedComponent :type Primitive%20Component%20Object%20Reference) (OtherActor :type Actor%20Object%20Reference) (OtherComp :type Primitive%20Component%20Object%20Reference) (OtherBodyIndex :type Integer) (bFromSweep :type Boolean) (SweepResult :type Hit%20Result%20Structure%20%28by%20ref%29))
  (bind _swordwidget (Variables|Default|GetSwordWidget))
  ;[0.15 0.15 0.15 0.5] 다가가면 위젯 나타남/ 멀어지면 사라짐
  (Widget|SetVisibility _swordwidget "Visible")
  ;[0.15 0.15 0.15 0.5] Text Fade in
  (UserInterface|Animation|PlayAnimation _swordwidget (Variables|/Game/Maps/MapAsset/sword/WB_SwordWidget.WB_SwordWidget_C|GetFadeIn _swordwidget) 0.0 1 "Forward" 1.0 false))

(event OnComponentEndOverlap(Capsule)
  (params (OverlappedComponent :type Primitive%20Component%20Object%20Reference) (OtherActor :type Actor%20Object%20Reference) (OtherComp :type Primitive%20Component%20Object%20Reference) (OtherBodyIndex :type Integer))
  (bind _swordwidget (Variables|Default|GetSwordWidget))
  ;[0.15 0.15 0.15 0.5] 다가가면 위젯 나타남/ 멀어지면 사라짐
  (UserInterface|Animation|PlayAnimation _swordwidget (Variables|/Game/Maps/MapAsset/sword/WB_SwordWidget.WB_SwordWidget_C|GetFadeOut _swordwidget) 0.0 1 "Forward" 1.0 false)
  ;[0.15 0.15 0.15 0.5] Text Fade out
  (Utilities|FlowControl|Delay 0.2)
  (Widget|SetVisibility _swordwidget "Hidden"))

(event Custom|StartBossBattle
  ;[0.15 0.15 0.15 0.5] 위젯이 떠있는 상태에서 보스전 시작 가능
  (if (Widget|IsVisible (Variables|Default|GetSwordWidget))
    (bind _asbp_my_game_mode_base (Utilities|Casting|CastToBP_MyGameModeBase (Game|GetGameMode)))
    (Variables|/Game/Game/BP_MyGameModeBase.BP_MyGameModeBase_C|SetIsBattleReady _asbp_my_game_mode_base true)))

(event EventBeginPlay
  ;[0.15 0.15 0.15 0.5] 위젯 화면에 추가
  (bind _returnvalue (UserInterface|CreateWidget "/Game/Maps/MapAsset/sword/WB_SwordWidget.WB_SwordWidget_C"))
  (bind _output_get (Variables|Default|SetSwordWidget _returnvalue))
  (UserInterface|Viewport|AddtoViewport _output_get 0))

(event Collision|EventActorBeginOverlap
  (params (OtherActor :type Actor%20Object%20Reference)))

(event EventTick
  (params (DeltaSeconds :type Float%20%28single-precision%29)))

(fn ConstructionScript)