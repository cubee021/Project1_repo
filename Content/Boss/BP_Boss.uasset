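; BP_Boss is a boss character with a health bar, a montage-driven attack and a ragdoll death.
; BeginPlay adds the WB_BossFIghtHealth widget to the viewport, and Tick writes Health to its bar every frame.
; Attack plays a montage once at a time; its notify fires a long debug-drawn sphere trace from AttackPos that damages the hit pawn.
; AnyDamage lowers Health, disabling movement and enabling mesh physics at zero.
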(event EventBeginPlay
  (bind _returnvalue (UserInterface|CreateWidget "/Game/Boss/WB_BossFIghtHealth.WB_BossFIghtHealth_C"))
  (UserInterface|Viewport|AddtoViewport _returnvalue 0)
  (Variables|Default|SetHealth%20UI _returnvalue))

(event EventAttack
  (bind _attack_pos (Variables|Default|GetAttack%20Pos))
  (bind _returnvalue (Transformation|GetWorldLocation _attack_pos))
  ;[0.15 0.15 0.15 0.5] Attack
  (if (not (Variables|Default|GetisAttacking?))
    (Animation|Montage|PlayMontage (Variables|Character|GetMesh) 0
      (:then
        (Variables|Default|SetisAttacking? true))
      (:OnCompleted
        (Variables|Default|SetisAttacking? false))
      (:OnNotifyBegin
        (bind (_outhit _returnvalue_2) (Collision|SphereTraceForObjects _returnvalue (+ _returnvalue (* (Math|Vector|GetForwardVector (Transformation|GetWorldRotation _attack_pos)) 3e+03)) 25.0 (Utilities|Array|MakeArray "ObjectTypeQuery3") false 0 "ForDuration" true "(R=1.000000,G=0.000000,B=0.000000,A=1.000000)" "(R=0.000000,G=1.000000,B=0.000000,A=1.000000)" 2.0))
        (if _returnvalue_2
          (Game|Damage|ApplyDamage (.HitActor (Collision|BreakHitResult _outhit)) 1e+01 0 0))))))

(event EventTick
  (params (DeltaSeconds :type Float%20%28single-precision%29))
  (Progress|SetPercent (Variables|/Game/Boss/WB_BossFIghtHealth.WB_BossFIghtHealth_C|GetHealthBar (Variables|Default|GetHealth%20UI)) (/ (Variables|Default|Gethealth) 1e+02)))

(event Game|Damage|EventAnyDamage
  (params (Damage :type Float%20%28single-precision%29) (DamageType :type Damage%20Type%20Object%20Reference) (InstigatedBy :type Controller%20Object%20Reference) (DamageCauser :type Actor%20Object%20Reference))
  ;[0.15 0.15 0.15 0.5] Health
  (Variables|Default|Sethealth (- (Variables|Default|Gethealth) Damage))
  (if (<= (Variables|Default|Gethealth) 0.0)
    (Pawn|Components|CharacterMovement|DisableMovement (Variables|Character|GetCharacterMovement))
    (Physics|SetSimulatePhysics (Variables|Character|GetMesh) true)))

(fn ConstructionScript)