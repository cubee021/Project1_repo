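; AI controller for the boss that cycles it through walking, turning and attacking with a Tick-driven state machine.
; It walks for a random time at 45 degrees off the player's direction, then interpolates yaw to face them.
; It rolls an attack count and picks each attack by player distance.
; Only Ice Charge runs through BPBossAttackComponent; the other attacks just print debug text.
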(event EventBeginPlay
  (Variables|Default|SetActionState "NewEnumerator1")
  (Variables|Default|SetRandomActionStateChangeTime (Math|Random|RandomFloatinRange 5.0 7.0))
  (bind _output_get (CallFunction|SetWalkDirection))
  (Variables|Default|SetBossWalkDirection _output_get))

(event EventTick
  (params (DeltaSeconds :type Float%20%28single-precision%29))
  (if (Utilities|Enum|Equal(Enum) (Variables|Default|GetActionState) "NewEnumerator1")
    (CallFunction|Walk)
    (elif (Utilities|Enum|Equal(Enum) (Variables|Default|GetActionState) "NewEnumerator5")
      (CallFunction|Rotate)
      (elif (Utilities|Enum|Equal(Enum) (Variables|Default|GetActionState) "NewEnumerator2")
        ;[0.15 0.15 0.15 0.5] AttackCount가 지정되어있지 않다면 지정
        (if (== (Variables|Default|GetTotAttackCount) 0)
          (bind _attackcount1 (CallFunction|SetAttackCount))
          (Variables|Default|SetTotAttackCount _attackcount1)
          (elif (< (Variables|Default|GetCurrentAttackCount) (Variables|Default|GetTotAttackCount))
            (CallFunction|Attack)
            (else
              (Variables|Default|SetActionState "NewEnumerator1")
              (Variables|Default|SetRandomActionStateChangeTime (Math|Random|RandomFloatinRange 5.0 7.0))
              (Variables|Default|SetWalkCurrentTime 0.0)
              (Variables|Default|SetCurrentAttackCount 0)
              (Variables|Default|SetTotAttackCount 0)
              (bind _output_get (CallFunction|SetWalkDirection))
              (bind _output_get_2 (Variables|Default|SetBossWalkDirection _output_get))
              (Development|PrintString (Utilities|String|ToString(Vector) _output_get_2)))))))))

(fn ConstructionScript)

(fn Walk
  ;[0.15 0.15 0.15 0.5] 2~4초 사이의 시간을 측정
  (bind _output_get (Variables|Default|SetWalkCurrentTime (+ (Variables|Default|GetWalkCurrentTime) (Utilities|Time|GetWorldDeltaSeconds))))
  (if (> _output_get (Variables|Default|GetRandomActionStateChangeTime))
    (Variables|Default|SetActionState "NewEnumerator5")
    (Development|PrintString "걷기끝@@@@@@@@@@@@@@@@@@@")
    (else
      (bind _returnvalue (Actor|GetActorOfClass "/Game/Boss/BP_Boss.BP_Boss_C"))
      (Transformation|SetActorTransform _returnvalue (Math|Transform|MakeTransform (+ (* (Utilities|Time|GetWorldDeltaSeconds) (* (Variables|Default|GetBossWalkDirection) (LocalVariables|GetBossWalkSpeed))) (Transformation|GetActorLocation _returnvalue)) (Math|Conversions|RotationFromXVector (Variables|Default|GetBossWalkDirection)) "1.000000,1.000000,1.000000") true)
      (Development|PrintString "걷는중"))))

(fn Attack
  (if (Utilities|Enum|Equal(Enum) (Variables|Default|GetAttackState) "NewEnumerator5")
    (bind _returnvalue (CallFunction|CalcDistancefromPlayer))
    (if (< _returnvalue 5e+02)
      ;[0.15 0.15 0.15 0.5] 할퀴기, 전방위 할퀴기
      (Variables|Default|SetAttackState (Utilities|Enum|ByteToEnumEBossAttackState (Math|Conversions|ToByte(Integer) (Math|Random|RandomIntegerinRange 1 2))))
      (else
        ;[0.15 0.15 0.15 0.5] 돌진, 바닥 내려찍기
        (Variables|Default|SetAttackState (Utilities|Enum|ByteToEnumEBossAttackState (Math|Conversions|ToByte(Integer) (Math|Random|RandomIntegerinRange 4 4))))))
    (else
      (switch Utilities|FlowControl|Switch|SwitchonEBossAttackState (Variables|Default|GetAttackState)
        (:NewEnumerator0
          (Development|PrintString "할퀴기" true true "(R=0.000000,G=0.660000,B=1.000000,A=1.000000)" 3.0))
        (:NewEnumerator1
          (Development|PrintString "전방위 할퀴기" true true "(R=0.000000,G=0.660000,B=1.000000,A=1.000000)" 3.0))
        (:NewEnumerator2
          (Development|PrintString "바닥 내려찍기!" true true "(R=0.000000,G=0.660000,B=1.000000,A=1.000000)" 3.0))
        (:NewEnumerator3
          (Development|PrintString "돌진!" true true "(R=0.000000,G=0.660000,B=1.000000,A=1.000000)" 3.0)
          (Default|IceCharge (Variables|Default|GetBP_BossAttackComponent)))))))

(fn CalcDistancefromPlayer
  (bind _returnvalue (Actor|GetActorOfClass "/Game/Boss/BP_Boss.BP_Boss_C"))
  (bind _returnvalue_2 (Actor|GetActorOfClass "/Game/Characters/Player/BP_CharacterBase.BP_CharacterBase_C"))
  (return (Math|Vector|VectorLength (- (Transformation|GetActorLocation _returnvalue) (Transformation|GetActorLocation _returnvalue_2)))))

(fn SetAttackCount
  (bind _returnvalue (Math|Random|RandomIntegerinRange 1 100))
  ;[0.15 0.15 0.15 0.5] 공격 1회 20%, 공격 2회 40%, 공격 3회 40%
  (if (<= _returnvalue 20)
    (LocalVariables|SetAttackCount 1)
    (return (LocalVariables|GetAttackCount))
    (elif (<= _returnvalue 60)
      (LocalVariables|SetAttackCount 2)
      (return (LocalVariables|GetAttackCount))
      (elif (<= _returnvalue 100)
        (LocalVariables|SetAttackCount 3)
        (return (LocalVariables|GetAttackCount))))))

(fn SetWalkDirection
  (bind _returnvalue (Actor|GetActorOfClass "/Game/Characters/Player/BP_CharacterBase.BP_CharacterBase_C"))
  (bind _returnvalue_2 (Actor|GetActorOfClass "/Game/Boss/BP_Boss.BP_Boss_C"))
  (bind _output_get (LocalVariables|SetTrueIsRight (Math|Random|RandomBool)))
  (if _output_get
    (LocalVariables|SetRotatedDir%20 (Math|Vector|RotateVectorAroundAxis (Math|Vector|Normalize (- (Transformation|GetActorLocation _returnvalue) (Transformation|GetActorLocation _returnvalue_2))) 45.0 "0.000000,0.000000,1.000000"))
    (else
      (LocalVariables|SetRotatedDir%20 (Math|Vector|RotateVectorAroundAxis (Math|Vector|Normalize (- (Transformation|GetActorLocation _returnvalue) (Transformation|GetActorLocation _returnvalue_2))) -45.0 "0.000000,0.000000,1.000000"))))
  (return (LocalVariables|GetRotatedDir%20)))

(fn SetAttackDirection
  (bind _returnvalue (Actor|GetActorOfClass "/Game/Characters/Player/BP_CharacterBase.BP_CharacterBase_C"))
  (bind _returnvalue_2 (Actor|GetActorOfClass "/Game/Boss/BP_Boss.BP_Boss_C"))
  (return (Math|Vector|Normalize (- (Transformation|GetActorLocation _returnvalue) (Transformation|GetActorLocation _returnvalue_2)))))

(fn Rotate
  (if (Variables|Default|GetIsRotated?)
    (Variables|Default|SetActionState "NewEnumerator2")
    (Variables|Default|SetIsRotated? false)
    (else
      (bind _rotatedirection (CallFunction|SetRotateDirection))
      (LocalVariables|SetRotateDirection _rotatedirection)
      (bind _returnvalue (Actor|GetActorOfClass "/Game/Boss/BP_Boss.BP_Boss_C"))
      (Transformation|SetActorRotation _returnvalue (Math|Rotator|MakeRotator 0.0 0.0 (.yaw (Math|Interpolation|RInterpTo (Transformation|GetActorRotation _returnvalue) (Math|Conversions|RotationFromXVector (LocalVariables|GetRotateDirection)) (Utilities|Time|GetWorldDeltaSeconds) 7.0))))
      (if (Utilities|Operators|EqualEqual (Math|Rotator|MakeRotator 0.0 0.0 (.yaw (Math|Interpolation|RInterpTo (Transformation|GetActorRotation _returnvalue) (Math|Conversions|RotationFromXVector (LocalVariables|GetRotateDirection)) (Utilities|Time|GetWorldDeltaSeconds) 7.0))) (Math|Rotator|MakeRotator 0.0 0.0 (.yaw (Math|Conversions|RotationFromXVector (LocalVariables|GetRotateDirection)))) 1.0)
        (Variables|Default|SetIsRotated? true)))))

(fn SetRotateDirection
  (bind _returnvalue (Actor|GetActorOfClass "/Game/Characters/Player/BP_CharacterBase.BP_CharacterBase_C"))
  (bind _returnvalue_2 (Actor|GetActorOfClass "/Game/Boss/BP_Boss.BP_Boss_C"))
  (return (Math|Vector|Normalize (- (Transformation|GetActorLocation _returnvalue) (Transformation|GetActorLocation _returnvalue_2)))))